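; BP_hittable is an actor in OfficeWars that takes damage from bullets and is destroyed when its health runs out.
; It starts alive with full health on BeginPlay, and each Hit from a BP_bullet subtracts a fixed amount.
; At zero health the Hit handler clears IsAlive, which Tick polls every frame to destroy the actor and print a Swedish death message.
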(event EventBeginPlay
  (Variables|Default|SetIsAlive true)
  (Variables|Default|SetHealth 1e+02))

(event EventHit
  (params (MyComp :type Primitive%20Component%20Object%20Reference) (Other :type Actor%20Object%20Reference) (OtherComp :type Primitive%20Component%20Object%20Reference) (bSelfMoved :type Boolean) (HitLocation :type Vector :default "0, 0, 0") (HitNormal :type Vector :default "0, 0, 0") (NormalImpulse :type Vector :default "0, 0, 0") (Hit :type Hit%20Result%20Structure%20%28by%20ref%29))
  (Utilities|Casting|CastToBP_bullet Other)
  (Variables|Default|SetHealth (- (Variables|Default|GetHealth) 1.0))
  (if (<= (Variables|Default|GetHealth) 0.0)
    (Variables|Default|SetIsAlive false)))

(event EventTick
  (params (DeltaSeconds :type Float%20%28single-precision%29))
  (if (not (Variables|Default|GetIsAlive))
    (Actor|DestroyActor)
    (Development|PrintString "död")))

(fn ConstructionScript)